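; BP_Block is a block actor that can be broken over time, with material-driven feedback as destruction progresses.
; On BeginPlay it creates a dynamic instance of M_Block on its Block component.
; StartDestroy plays a timeline from the start, feeding the material's DestroyAmount parameter and destroying the actor when finished.
; StopDestroy cancels this by resetting the parameter and stopping the timeline, so progress is not kept.
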(event Custom|StopDestroy
  (Rendering|Material|SetScalarParameterValue (Variables|Default|GetBlockMat) "DestroyAmount" 0.0 :!class /Script/Engine.MaterialInstanceDynamic)
  (bind _destroyamount (Timeline|DestroyTimelne Stop)
    (:Update
      (Rendering|Material|SetScalarParameterValue (Variables|Default|GetBlockMat) "DestroyAmount" _destroyamount :!class /Script/Engine.MaterialInstanceDynamic))
    (:Finished
      (Actor|DestroyActor))))

(event Custom|StartDestroy
  (bind _destroyamount (Timeline|DestroyTimelne PlayFromStart)
    (:Update
      (Rendering|Material|SetScalarParameterValue (Variables|Default|GetBlockMat) "DestroyAmount" _destroyamount :!class /Script/Engine.MaterialInstanceDynamic))
    (:Finished
      (Actor|DestroyActor))))

(event EventBeginPlay
  (bind _returnvalue (Rendering|Material|CreateDynamicMaterialInstance (Variables|Default|GetBlock) 0 "/Game/Materials/M_Block.M_Block" "None" :!class /Script/Engine.PrimitiveComponent))
  (Variables|Default|SetBlockMat _returnvalue))

(fn ConstructionScript)